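; GameCamera is the game's camera actor, which becomes player 0's view target and smoothly follows a target, by default the GameCharacter.
; On BeginPlay it uses its Character reference, or the first GameCharacter found in the level, as CameraTarget.
; Each Tick lerps its location toward the target using BetterLerpAlpha, easing more gently for a GameCharacter, where it tracks the Character reference, than for other targets.
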(event `self.ReceiveBeginPlay`
  (`|ExecutionSequence`
    (:`then_0`
      (`PlayerController.SetViewTargetWithBlend` (`GameplayStatics.GetPlayerController` 0) self 0.0 "VTBlend_Linear" 0.0 false))
    (:`then_1`
      (`/Engine/EditorBlueprintResources/StandardMacros.IsValid` (`self.character`)
        (:`Is Valid`
          (set `self.camera target` (`self.character`)))
        (:`Is Not Valid`
          (bind _outactors (`GameplayStatics.GetAllActorsOfClass` "/Game/Blueprints/GameCharacter.GameCharacter_C"))
          (set `self.character` (`|GetArrayItem` _outactors))
          (set `self.camera target` (`self.character`)))))))

(event `self.ReceiveTick`
  (params (DeltaSeconds :type "Float (single-precision)"))
  (bind _asgame_character (cast `/Game/Blueprints/GameCharacter` (`self.camera target`))
    (:`then`
      (`self.K2_SetActorLocation` (`KismetMathLibrary.VLerp` (`self.K2_GetActorLocation`) (+ (`self.K2_GetActorLocation` (`self.character`)) (0.0 0.0 0.0)) (`/Game/Blueprints/maths.better lerp alpha` 0.03))))
    (:`CastFailed`
      (`self.K2_SetActorLocation` (`KismetMathLibrary.VLerp` (`self.K2_GetActorLocation`) (`self.K2_GetActorLocation` (`self.camera target`)) (`/Game/Blueprints/maths.better lerp alpha` 0.05))))))

(fn `UserConstructionScript`)