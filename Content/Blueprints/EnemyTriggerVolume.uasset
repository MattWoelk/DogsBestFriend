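; Trigger volume that activates a set of enemy spawners once, then destroys itself.
; On overlap it ignores any GameCharacter; another actor that casts to Human makes it call Spawn on every entry in its Spawners array.
; The construction script keeps the root at unit scale and sizes the box footprint from the X and Y variables, leaving Z scale at one.
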(event `self.ReceiveActorBeginOverlap`
  (params (OtherActor :type "Actor Object Reference"))
  (cast `/Game/Blueprints/GameCharacter` OtherActor
    (:`CastFailed`
      (cast `/Game/Blueprints/Human` OtherActor)
      (for _array_element (`self.spawners`)
        (`/Game/Blueprints/EnemySpawner.spawn!` _array_element))
      (`self.K2_DestroyActor`))))

(fn `UserConstructionScript`
  (`SceneComponent.SetWorldScale3D` (`self.DefaultSceneRoot`) (1.0 1.0 1.0))
  (`SceneComponent.SetWorldScale3D` (`self.Box`) (`KismetMathLibrary.MakeVector` (* (`self.x`) 0.01) (* (`self.y`) 0.01) 1.0)))