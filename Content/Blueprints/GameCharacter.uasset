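; Player dog pawn that walks, barks, carries an apple to feed humans, and can be petted by them.
; A Walking/Barking/BeingPet state gates input and drives the procedural bounce, sprite flip and flickering bark texture.
; Barking briefly enables physics on every Enemy and applies a radial impulse from below the dog.
; Overlaps handle pickups and humans, and switch the GameCamera target between the current Arena and the dog.
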(event `self.ReceiveActorEndOverlap`
  (params (OtherActor :type "Actor Object Reference"))
  (cast `/Game/Blueprints/Arena` OtherActor)
  (set `/Game/Blueprints/GameCamera.camera target` self (`self.game camera`)))

(event `get pickup`
  (`SceneComponent.SetHiddenInGame` (`self.backpack plane`) false true)
  (set `self.has apple` true))

(event `InputAction|bark`
  (params (Key :type "Key Structure"))
  ;[1 1 1] Bark
  (:`Pressed`
    (`self.can move`
      (:`true`
        (`|ExecutionSequence`
          (:`then_0`
            (bind _outactors (`GameplayStatics.GetAllActorsOfClass` "/Game/Blueprints/Enemy.Enemy_C"))
            (for _array_element _outactors
              (`/Game/Blueprints/Enemy.enable physics briefly` _array_element)
              (`PrimitiveComponent.AddRadialImpulse` (`Character.CapsuleComponent` _array_element) (+ (`self.K2_GetActorLocation`) (0.0 0.0 -100.0)) 10000.0 500.0 "RIF_Constant" true)
              (`KismetSystemLibrary.PrintString` (`KismetSystemLibrary.GetDisplayName` _array_element))))
          (:`then_1`
            (set `self.state` "NewEnumerator1")
            (`SceneComponent.SetHiddenInGame` (`self.bork plane`) false false)
            (`KismetSystemLibrary.Delay` 1.0)
            (`SceneComponent.SetHiddenInGame` (`self.bork plane`) true false :!label _label)
            (set `self.state` "NewEnumerator0"))
          (:`then_2`
            (bind (_direction _jump_z _jump_y) (`Timeline|bark jump` :!via `PlayFromStart`)
              (:`Update`
                (`SceneComponent.K2_SetRelativeLocation` (`self.character`) (`KismetMathLibrary.MakeVector` 0.0 (* _jump_y 0.0) (* _jump_z 50.0)) false false)))))))))

(event `self.ReceiveActorBeginOverlap`
  (params (OtherActor :type "Actor Object Reference"))
  (bind _asarena (cast `/Game/Blueprints/Arena` OtherActor)
    (:`then`
      (set `/Game/Blueprints/GameCamera.camera target` _asarena (`self.game camera`)))
    (:`CastFailed`
      (bind _aspickup (cast `/Game/Blueprints/pickup` OtherActor)
        (:`then`
          (`self.get pickup`)
          (`self.K2_DestroyActor` _aspickup))
        (:`CastFailed`
          (bind _ashuman (cast `/Game/Blueprints/Human` OtherActor))
          (if (`self.has apple`)
            (`/Game/Blueprints/Human.eat` _ashuman)
            (`self.drop pickup`)
            (elif (`|EnumEquality` (`/Game/Blueprints/Human.state` _ashuman) "NewEnumerator1")
              (`self.stop barking`)
              (`/Game/Blueprints/Human.pet the dog` _ashuman)
              (`SceneComponent.SetHiddenInGame` (`self.Plane`) true false)
              (set `self.state` "NewEnumerator2")
              (`KismetSystemLibrary.Delay` 2.0)
              (set `self.state` "NewEnumerator0")
              (`SceneComponent.SetHiddenInGame` (`self.Plane`) false false))))))))

(event `self.ReceiveBeginPlay`
  (bind _outactors (`GameplayStatics.GetAllActorsOfClass` "/Game/Blueprints/GameCamera.GameCamera_C"))
  (set `self.game camera` (`|GetArrayItem` _outactors)))

(event `drop pickup`
  (`SceneComponent.SetHiddenInGame` (`self.backpack plane`) true true)
  (set `self.has apple` false))

(event `stop barking`
  ;[1 1 1] Bark
  (goto _label))

(event `InputAxis|move northsouth`
  (params (AxisValue :type "Float (single-precision)"))
  (`self.can move`
    (:`true`
      (`PawnMovementComponent.AddInputVector` (`self.FloatingPawnMovement`) (`KismetMathLibrary.MakeVector` AxisValue) false))))

(event `InputAxis|move eastwest`
  (params (AxisValue :type "Float (single-precision)"))
  (`self.can move`
    (:`true`
      (`PawnMovementComponent.AddInputVector` (`self.FloatingPawnMovement`) (`KismetMathLibrary.MakeVector` 0.0 AxisValue) false))))

(event `self.ReceiveTick`
  (params (DeltaSeconds :type "Float (single-precision)"))
  (bind _returnvalue (`PawnMovementComponent.GetLastInputVector` (`self.FloatingPawnMovement`)))
  (switch `/Game/Blueprints/states_dog` (`self.state`)
    (:`NewEnumerator0`
      ;[1 1 1] Walking
      (`|ExecutionSequence`
        (:`then_0`
          ;[1 1 1] bounce
          (`SceneComponent.K2_SetRelativeLocation` (`self.character`) (`KismetMathLibrary.MakeVector` 0.0 0.0 (+ (* (`KismetMathLibrary.VSize` (`PawnMovementComponent.GetLastInputVector` (`self.FloatingPawnMovement`))) (`KismetMathLibrary.Abs` (`KismetMathLibrary.DegSin` (* (`GameplayStatics.GetTimeSeconds`) 360.0 3.0))) 25.0) 0.0)) false false))
        (:`then_1`
          ;[1 1 1] flip
          (if (> (`KismetMathLibrary.Abs` (.y _returnvalue)) 0.2)
            (`SceneComponent.K2_SetRelativeRotation` (`self.Plane`) (`KismetMathLibrary.MakeRotator` 0.0 (`KismetMathLibrary.SelectFloat` 180.0 0.0 (> (`KismetMathLibrary.Dot_VectorVector` (`KismetMathLibrary.Normal` _returnvalue) (0.0 1.0 0.0)) 0.0))) false false)))))
    (:`NewEnumerator1`
      ;[1 1 1] Barking
      (`MaterialInstanceDynamic.SetTextureParameterValue` (`self.bork material`) "texture" (select `bool` (> (`KismetMathLibrary.Fraction` (* (`GameplayStatics.GetTimeSeconds`) 1.0)) 0.5) :`false` "/Game/Sprites/bork_1.bork_1" :`true` "/Game/Sprites/bork_2.bork_2" :!type "Texture Object Reference")))))

(fn `UserConstructionScript`
  (bind _returnvalue (`PrimitiveComponent.CreateDynamicMaterialInstance` (`self.bork plane`) 0 "/Game/Materials/bork_mat.bork_mat" "None"))
  (bind _output_get (set `self.bork material` _returnvalue))
  (`MaterialInstanceDynamic.SetTextureParameterValue` _output_get "texture" "/Game/Sprites/bork_1.bork_1"))