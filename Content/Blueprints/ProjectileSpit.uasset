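; ProjectileSpit is a spit projectile actor, shown as an animated sprite on a plane.
; The construction script creates a dynamic material instance from Character_mat and sets the first spit texture.
; Tick drives a time-based flipbook by swapping the texture parameter between three spit frames, looping three times a second.
; It also resets the plane to a fixed world rotation every frame, keeping its orientation independent of the actor.
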(event `self.ReceiveTick`
  (params (DeltaSeconds :type "Float (single-precision)"))
  (bind _returnvalue (`KismetMathLibrary.Fraction` (* (`GameplayStatics.GetTimeSeconds`) 3.0)))
  (`|ExecutionSequence`
    (:`then_0`
      ;[1 1 1] spit flipbook
      (`MaterialInstanceDynamic.SetTextureParameterValue` (`self.material`) "texture" (select `bool` (> _returnvalue 0.66) :`false` (select `bool` (> _returnvalue 0.33) :`false` "/Game/Sprites/spit_2.spit_2" :`true` "/Game/Sprites/spit_3.spit_3" :!type "Texture Object Reference") :`true` "/Game/Sprites/spit_1.spit_1")))
    (:`then_1`
      (`SceneComponent.K2_SetWorldRotation` (`self.Plane`) (struct :`Yaw` 90.0 :`Roll` 90.0) false false))))

(fn `UserConstructionScript`
  (bind _returnvalue (`PrimitiveComponent.CreateDynamicMaterialInstance` (`self.Plane`) 0 "/Game/Materials/character_mat.character_mat" "None"))
  (bind _output_get (set `self.material` _returnvalue))
  (`MaterialInstanceDynamic.SetTextureParameterValue` _output_get "texture" "/Game/Sprites/spit_1.spit_1"))