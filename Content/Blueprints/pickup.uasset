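; Pickup actor whose look is set by a texture and a tint, with no collection logic in this graph.
; The construction script creates one dynamic instance of Pickup_mat, applies both parameters and shares it between two plane components.
; Tick destroys the actor once it drops below a fixed world height.
; BeginPlay and overlap events are empty, disabled stubs.
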(event `self.ReceiveTick`
  (params (DeltaSeconds :type "Float (single-precision)"))
  (bind (_returnvalue_x _returnvalue_y _returnvalue_z) (`KismetMathLibrary.BreakVector` (`self.K2_GetActorLocation`)))
  (if (< _returnvalue_z -500.0)
    (`self.K2_DestroyActor`)))

(fn `UserConstructionScript`
  (bind _returnvalue (`PrimitiveComponent.CreateDynamicMaterialInstance` (`self.Plane`) 0 "/Game/Materials/pickup_mat.pickup_mat" "None"))
  (bind _output_get (set `self.material` _returnvalue))
  (`MaterialInstanceDynamic.SetTextureParameterValue` _output_get "texture" (`self.texture`))
  (`MaterialInstanceDynamic.SetVectorParameterValue` _output_get "tint" (`self.tint`))
  (`PrimitiveComponent.SetMaterial` (`self.Plane1`) 0 (`self.material`)))