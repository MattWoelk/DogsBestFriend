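; Human is an AI pawn drawn as a textured plane that follows a target actor, defaulting to the first GameCharacter found.
; Tick reissues AIMoveTo toward the target and pins the plane to a fixed world rotation so the image does not turn with movement.
; The construction script applies the per-instance Texture through a dynamic material.
; A separate event enables capsule physics, then switches it off after a short retriggerable delay.
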(event `self.ReceiveBeginPlay`
  (`/Engine/EditorBlueprintResources/StandardMacros.IsValid` (`self.target`)
    (:`Is Not Valid`
      (bind _outactors (`GameplayStatics.GetAllActorsOfClass` "/Game/Blueprints/GameCharacter.GameCharacter_C"))
      (set `self.target` (`|GetArrayItem` _outactors)))))

(event `self.ReceiveTick`
  (params (DeltaSeconds :type "Float (single-precision)"))
  (`|ExecutionSequence`
    (:`then_0`
      (`|AIMoveTo` self (0.0 0.0 0.0) (`self.target`)))
    (:`then_1`
      (`SceneComponent.K2_SetWorldRotation` (`self.Plane`) (struct :`Yaw` -90.0 :`Roll` 90.0) false false))))

(event `enable physics briefly`
  (bind _capsulecomponent (`self.CapsuleComponent`))
  (`PrimitiveComponent.SetSimulatePhysics` _capsulecomponent true)
  (`KismetSystemLibrary.RetriggerableDelay` 1.0)
  (`PrimitiveComponent.SetSimulatePhysics` _capsulecomponent false))

(fn `UserConstructionScript`
  (bind _returnvalue (`PrimitiveComponent.CreateDynamicMaterialInstance` (`self.Plane`) 0 "/Game/Materials/character_mat.character_mat" "None"))
  (bind _output_get (set `self.material` _returnvalue))
  (`MaterialInstanceDynamic.SetTextureParameterValue` _output_get "texture" (`self.texture`)))