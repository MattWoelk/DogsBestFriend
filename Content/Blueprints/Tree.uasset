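; Tree is a scenery actor that can act as a tree or a bush, shaking its foliage and optionally dropping an apple pickup.
; The construction script creates a dynamic material with an apple or bare texture, and bush mode puts it on the trunk plane and hides the leaves.
; The shaketree event plays a timeline that wobbles the visible plane and spawns one apple if none exists.
; A flip event rotates the root by 180 degrees.
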(event `flip`
  (`SceneComponent.K2_AddWorldRotation` (`self.DefaultSceneRoot`) (struct :`Yaw` 180.0) false false))

(event `shake tree`
  (`|ExecutionSequence`
    (:`then_0`
      (bind (_direction _x _y) (`Timeline|shake leaves` :!via `PlayFromStart`)
        (:`Update`
          (`SceneComponent.K2_SetRelativeLocation` (select `bool` (`self.is bush?`) :`false` (`self.leaves plane`) :`true` (`self.trunk plane`) :!type "SceneComponent Object Reference") (+ (* (`KismetMathLibrary.MakeVector` _x 0.0 _y) 20.0) (select `bool` (`self.is bush?`) :`false` (`KismetMathLibrary.MakeVector` 0.28837 -0.100058 112.311493) :`true` (`KismetMathLibrary.MakeVector` 0.0 0.0 25.0))) false false))))
    (:`then_1`
      (if (`self.has apples?`)
        ;[1 1 1] if we have no apple, drop one
        (`/Engine/EditorBlueprintResources/StandardMacros.IsValid` (`self.apple`)
          (:`Is Not Valid`
            (bind _returnvalue (`|SpawnActorFromClass` "/Game/Blueprints/pickup.pickup_C" (`KismetMathLibrary.MakeTransform` (`KismetMathLibrary.TransformLocation` (`self.GetTransform`) (`self.apple spot`))) "Undefined" "OverrideRootScale" null "NewEnumerator0" null))
            (set `self.apple` _returnvalue)))))))

(fn `UserConstructionScript`
  (`|ExecutionSequence`
    (:`then_0`
      (bind _returnvalue (`PrimitiveComponent.CreateDynamicMaterialInstance` (`self.leaves plane`) 0 "/Game/Materials/character_mat.character_mat" "None"))
      (bind _output_get (set `self.material` _returnvalue))
      (`MaterialInstanceDynamic.SetTextureParameterValue` _output_get "texture" (select `bool` (`self.has apples?`) :`false` "/Game/Sprites/tree_top_-_no_apples.tree_top_-_no_apples" :`true` "/Game/Sprites/tree_top.tree_top" :!type "Texture Object Reference")))
    (:`then_1`
      (if (`self.is bush?`)
        (`PrimitiveComponent.SetMaterial` (`self.trunk plane`) 0 (`self.material`))
        (`SceneComponent.SetVisibility` (`self.leaves plane`) false true)
        (`SceneComponent.K2_SetRelativeLocation` (`self.trunk plane`) (0.0 0.0 25.0) false false)))))