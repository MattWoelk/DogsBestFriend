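; Light actor that continuously moves its PointLight component around its origin in a wandering pattern.
; Each Tick sets the light's relative location from three sine waves of game time, phase-shifted per axis by fixed time offsets.
; SpeedFactor scales the wave frequency and Amplitude scales how far the light travels.
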(event `self.ReceiveTick`
  (params (DeltaSeconds :type "Float (single-precision)"))
  (`SceneComponent.K2_SetRelativeLocation` (`self.PointLight`) (* (`KismetMathLibrary.MakeVector` (`KismetMathLibrary.Sin` (* (`GameplayStatics.GetTimeSeconds`) (`self.speed factor`))) (`KismetMathLibrary.Sin` (* (+ (`GameplayStatics.GetTimeSeconds`) 1.32984) (`self.speed factor`))) (`KismetMathLibrary.Sin` (* (+ (`GameplayStatics.GetTimeSeconds`) 10.23) (`self.speed factor`)))) (`self.amplitude`)) false false))

(fn `UserConstructionScript`)