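; Enemy character, either Rat or Snake, that chases a Human and attacks with melee bites or spit projectiles respectively.
; Tick runs a Walking/Attacking/Stunned state machine, using AI MoveTo, per-type ranges and a gated attack cooldown.
; A textured plane is animated procedurally with sine movement, flipping and frame swaps.
; Stun briefly enables capsule physics; damage shakes and tints the plane, and death spawns a corpse.
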(event `self.ReceiveBeginPlay`
  (`/Engine/EditorBlueprintResources/StandardMacros.IsValid` (`self.target`)
    (:`Is Not Valid`
      (bind _outactors (`GameplayStatics.GetAllActorsOfClass` "/Game/Blueprints/Human.Human_C"))
      (set `self.target` (`|GetArrayItem` _outactors)))))

(event `self.ReceiveTick`
  (params (DeltaSeconds :type "Float (single-precision)"))
  (bind _returnvalue (`self.K2_GetActorLocation`))
  (bind _type (`self.type`))
  (bind _velocity (`MovementComponent.Velocity` (`self.CharacterMovement`)))
  (`|ExecutionSequence`
    (:`then_0`
      (if (`|EnumInequality` (`self.state`) "NewEnumerator0")
        (`NavMovementComponent.StopActiveMovement` (`self.CharacterMovement`))))
    (:`then_1`
      (switch `/Game/Blueprints/states_enemy` (`self.state`)
        (:`NewEnumerator0`
          (`|ExecutionSequence`
            (:`then_0`
              ;[1 1 1] move to target
              (`|AIMoveTo` self (0.0 0.0 0.0) (`self.target`)
                (:`then`
                  ;[1 1 1] close enough to attack?
                  (if (< (`self.GetDistanceTo` (`self.target`) self) (select `/Game/Blueprints/enemy_types` (`self.type`) :`NewEnumerator0` 100.0 :`NewEnumerator1` 500.0 :!type "Float (single-precision)"))
                    (set `self.state` "NewEnumerator1")))))
            (:`then_1`
              ;[1 1 1] Walk Animation
              (`SceneComponent.K2_SetRelativeLocation` (`self.Plane`) (select `/Game/Blueprints/enemy_types` (`self.type`) :`NewEnumerator0` (`KismetMathLibrary.MakeVector` 0.0 (+ (* (`KismetMathLibrary.VSize` (`MovementComponent.Velocity` (`self.CharacterMovement`))) (`KismetMathLibrary.Abs` (`KismetMathLibrary.DegSin` (* (`GameplayStatics.GetTimeSeconds`) 360.0 4.0))) -0.05) 0.0)) :`NewEnumerator1` (`KismetMathLibrary.MakeVector` (+ (* (`KismetMathLibrary.VSize` (`MovementComponent.Velocity` (`self.CharacterMovement`))) (`KismetMathLibrary.DegSin` (* (`GameplayStatics.GetTimeSeconds`) 360.0 1.0)) 0.1) 0.0))) false false))
            (:`then_2`
              ;[1 1 1] Flip
              (if (> (`KismetMathLibrary.Abs` (.y _velocity)) 0.2)
                (`SceneComponent.K2_SetWorldRotation` (`self.Plane`) (`KismetMathLibrary.MakeRotator` 90.0 0.0 (`KismetMathLibrary.SelectFloat` 90.0 -90.0 (> (`KismetMathLibrary.Dot_VectorVector` (`KismetMathLibrary.Normal` _velocity) (0.0 1.0 0.0)) 0.0))) false false)))
            (:`then_3`
              ;[1 1 1] texture animation
              (`MaterialInstanceDynamic.SetTextureParameterValue` (`self.material`) "texture" (select `bool` (> (`KismetMathLibrary.Fraction` (* (`GameplayStatics.GetTimeSeconds`) (select `/Game/Blueprints/enemy_types` (`self.type`) :`NewEnumerator0` 3.0 :`NewEnumerator1` 1.3 :!type "Float (single-precision)"))) 0.5) :`false` (select `/Game/Blueprints/enemy_types` _type :`NewEnumerator0` "/Game/Sprites/rat_1.rat_1" :`NewEnumerator1` "/Game/Sprites/snake_1.snake_1" :!type "Texture Object Reference") :`true` (select `/Game/Blueprints/enemy_types` _type :`NewEnumerator0` "/Game/Sprites/rat_2.rat_2" :`NewEnumerator1` "/Game/Sprites/snake_2.snake_2" :!type "Texture Object Reference"))))))
        (:`NewEnumerator1`
          ;[1 1 1] close enough to keep attacking?
          (if (< (`self.GetDistanceTo` (`self.target`) self) (select `/Game/Blueprints/enemy_types` (`self.type`) :`NewEnumerator0` 120.0 :`NewEnumerator1` 520.0 :!type "Float (single-precision)"))
            ;[1 1 1] do damage or shoot projectile every so often
            (`/Engine/EditorBlueprintResources/StandardMacros.Gate` false :!label _label
              (:`Exit`
                (`|ExecutionSequence`
                  (:`then_0`
                    (switch `/Game/Blueprints/enemy_types` (`self.type`)
                      (:`NewEnumerator0`
                        ;;[1 1 1] Rat attack
                        (bind _ashuman (cast `/Game/Blueprints/Human` (`self.target`)))
                        (`/Game/Blueprints/Human.take damage` _ashuman 0.05))
                      (:`NewEnumerator1`
                        (`|SpawnActorFromClass` "/Game/Blueprints/ProjectileSpit.ProjectileSpit_C" (`KismetMathLibrary.MakeTransform` _returnvalue (`KismetMathLibrary.Conv_VectorToRotator` (- (`self.K2_GetActorLocation` (`self.target`)) _returnvalue))) "Undefined" "OverrideRootScale" null null))))
                  (:`then_1`
                    (goto _label :!via `Close`))
                  (:`then_2`
                    (`KismetSystemLibrary.Delay` (select `/Game/Blueprints/enemy_types` (`self.type`) :`NewEnumerator0` 1.5 :`NewEnumerator1` 3.0 :!type "Float (single-precision)"))
                    (goto _label :!via `Open`))
                  (:`then_3`
                    (`MaterialInstanceDynamic.SetTextureParameterValue` (`self.material`) "texture" (select `/Game/Blueprints/enemy_types` (`self.type`) :`NewEnumerator0` "/Game/Sprites/rat_up_2.rat_up_2" :`NewEnumerator1` "/Game/Sprites/snake_attack_2.snake_attack_2" :!type "Texture Object Reference"))
                    (`KismetSystemLibrary.Delay` 0.3)
                    (`MaterialInstanceDynamic.SetTextureParameterValue` (`self.material`) "texture" (select `/Game/Blueprints/enemy_types` (`self.type`) :`NewEnumerator0` "/Game/Sprites/rat_up_1.rat_up_1" :`NewEnumerator1` "/Game/Sprites/snake_attack_1.snake_attack_1" :!type "Texture Object Reference"))))))
            (else
              (set `self.state` "NewEnumerator0"))))))
    (:`then_2`
      (`SceneComponent.K2_SetWorldRotation` (`self.character`) (struct :`Yaw` -90.0 :`Roll` 90.0) false false))))

(event `stun briefly`
  ;[1 1 1] stun
  (`|ExecutionSequence`
    (:`then_0`
      (set `self.state` "NewEnumerator2")
      (`PrimitiveComponent.SetSimulatePhysics` (`self.CapsuleComponent`) true)
      (`MaterialInstanceDynamic.SetTextureParameterValue` (`self.material`) "texture" (select `/Game/Blueprints/enemy_types` (`self.type`) :`NewEnumerator0` "/Game/Sprites/rat_1.rat_1" :`NewEnumerator1` "/Game/Sprites/snake_1.snake_1" :!type "Texture Object Reference")))
    (:`then_1`
      (`KismetSystemLibrary.RetriggerableDelay` 1.0)
      (set `self.state` "NewEnumerator0")
      (`PrimitiveComponent.SetSimulatePhysics` (`self.CapsuleComponent`) false))))

(event `take damage`
  (params (damage :type "Float (double-precision)"))
  (bind (_returnvalue_x _returnvalue_y _returnvalue_z) (`KismetMathLibrary.BreakVector` (`KismetMathLibrary.MakeVector` (+ (- 1.0 (`self.health`)) 1.0) 1.0 1.0)))
  ;[1 1 1] take damage
  (set `self.health` (`KismetMathLibrary.FMax` (- (`self.health`) damage)))
  (`|ExecutionSequence`
    (:`then_0`
      (bind (_direction _x _y) (`Timeline|Timeline_0` :!via `PlayFromStart`)
        (:`Update`
          (`SceneComponent.K2_SetRelativeLocation` (`self.Plane`) (+ (* (`KismetMathLibrary.MakeVector` _x _y) 40.0) (0.0 0.0 0.0)) false false))))
    (:`then_1`
      (if (<= (`self.health`) 0.0)
        (`|SpawnActorFromClass` "/Game/Blueprints/dead_animal.dead_animal_C" (`KismetMathLibrary.MakeTransform` (+ (`self.K2_GetActorLocation`) (0.0 0.0 -90.0))) "Undefined" "OverrideRootScale" null (select `/Game/Blueprints/enemy_types` (`self.type`) :`NewEnumerator0` "/Game/Sprites/rat_dead.rat_dead" :`NewEnumerator1` "/Game/Sprites/snake_dead.snake_dead" :!type "Texture Object Reference") null)
        (`self.K2_DestroyActor`)))
    (:`then_2`
      (`MaterialInstanceDynamic.SetVectorParameterValue` (`self.material`) "tint" (make `LinearColor` _returnvalue_x _returnvalue_y _returnvalue_z 1.0)))))

(fn `UserConstructionScript`
  (bind _returnvalue (`PrimitiveComponent.CreateDynamicMaterialInstance` (`self.Plane`) 0 "/Game/Materials/character_mat.character_mat" "None"))
  (bind _output_get (set `self.material` _returnvalue))
  (`MaterialInstanceDynamic.SetTextureParameterValue` _output_get "texture" (select `/Game/Blueprints/enemy_types` (`self.type`) :`NewEnumerator0` "/Game/Sprites/rat_1.rat_1" :!type "Texture Object Reference")))